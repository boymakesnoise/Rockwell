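; Cart actor that rides back and forth along the spline of a referenced track, starting Still.
; Tick reads MovementState to play, reverse or stop the CartMover timeline, with play rate derived from Duration and start time seeded by StartOffset.
; Timeline updates map Alpha to spline distance to set location and rotation.
; Finishing returns the state to Still, while SwitchDir is updated from movement or the end reached.
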(event `self.ReceiveBeginPlay`
  (bind _myspline (`/Game/Blueprints/BP_SplineMesh.MySpline` (`self.TrackReference`)))
  (`self.K2_SetActorLocationAndRotation` (`SplineComponent.GetLocationAtDistanceAlongSpline` _myspline 0.0 "World") (`SplineComponent.GetRotationAtDistanceAlongSpline` _myspline 0.0 "World"))
  (set `self.MovementState` "NewEnumerator0")
  (`TimelineComponent.SetNewTime` (`self.CartMover`) (`self.StartOffset`)))

(event `self.ReceiveTick`
  (params (DeltaSeconds :type "Float (single-precision)"))
  (bind _myspline (`/Game/Blueprints/BP_SplineMesh.MySpline` (`self.TrackReference`)))
  (switch `/Game/Blueprints/E_CartDirection` (`self.MovementState`)
    (:`NewEnumerator1`
      (`self.MoveCartForwards`)
      (set `self.CanStartCart` false)
      (set `self.SwitchDir` 1 :!label _label))
    (:`NewEnumerator0`
      ;[1 1 1] Move Cart
      (bind (_direction _alpha) (`Timeline|CartMover` :!via `Stop` :!label _label_2)
        (:`Update`
          (bind _output_get (set `self.Alpha` _alpha))
          (bind _returnvalue (`KismetMathLibrary.Lerp` 0.0 (`SplineComponent.GetSplineLength` _myspline) _output_get))
          (`self.K2_SetActorLocationAndRotation` (`SplineComponent.GetLocationAtDistanceAlongSpline` _myspline _returnvalue "World") (`SplineComponent.GetRotationAtDistanceAlongSpline` _myspline _returnvalue "World")))
        (:`Finished`
          (bind _output_get_2 (set `self.MovementState` "NewEnumerator0"))
          (`KismetSystemLibrary.PrintString` (`|GetEnumeratorNameAsString` _output_get_2))
          (if (== (`self.Alpha`) 0.0)
            (set `self.SwitchDir` -1 :!label _label_3)
            (else
              (goto _label))))))
    (:`NewEnumerator2`
      (`self.MoveCartBackwards`)
      (goto _label_3))))

(event `MoveCartForwards`
  ;[1 1 1] Move Cart
  (`TimelineComponent.SetPlayRate` (`self.CartMover`) (/ 1.0 (`self.Duration`)))
  (goto _label_2))

(event `MoveCartBackwards`
  (`TimelineComponent.SetPlayRate` (`self.CartMover`) (/ 1.0 (`self.Duration`)))
  (goto _label_2 :!via `Reverse`))

(fn `UserConstructionScript`)