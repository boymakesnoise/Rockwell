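; Player-controlled crane with a switchable magnet, in a timed game that pauses when the countdown reaches zero.
; Input axes swing the arm, slide the cable mount along it and set cable length, applied each Tick as a physics constraint limit.
; While magnetic, ApplyInfluence pushes or pulls overlapping components with squared distance falloff, using material comparison as polarity.
; A Delay on Tick drives the countdown; the magnet's reaction force is left unconnected.
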(event `InputAxis|CraneRight`
  (params (AxisValue :type "Float (single-precision)"))
  (bind (_returnvalue_roll _returnvalue_pitch _returnvalue_yaw) (`KismetMathLibrary.BreakRotator` (`SceneComponent.K2_GetComponentRotation` (`self.PivotPoint`))))
  ;[1 1 1] Swing the arm
  (`SceneComponent.K2_SetWorldRotation` (`self.PivotPoint`) (`KismetMathLibrary.MakeRotator` 0.0 0.0 (+ _returnvalue_yaw (* AxisValue 0.2))) false false))

(event `InputAxis|CraneForward`
  (params (AxisValue :type "Float (single-precision)"))
  (bind _cone (`self.Cone`))
  (bind (_relativelocation_x _relativelocation_y _relativelocation_z) (`KismetMathLibrary.BreakVector` (`SceneComponent.RelativeLocation` _cone)))
  ;[1 1 1] Cable along arm
  (`SceneComponent.K2_SetRelativeLocation` _cone (`KismetMathLibrary.MakeVector` (`KismetMathLibrary.FClamp` (+ _relativelocation_x (* AxisValue 0.2)) -22.0 43.0) _relativelocation_y _relativelocation_z) false false))

(event `InputAxis|MagnetUpDown`
  (params (AxisValue :type "Float (single-precision)"))
  ;[1 1 1] Set Cable Length
  (set `self.CableLength` (`KismetMathLibrary.FClamp` (+ (* AxisValue 10.0) (`self.CableLength`)) 25.0 750.0)))

(event `InputAction|ToggleMagnet`
  (params (Key :type "Key Structure"))
  (:`Pressed`
    (if (`self.Magnetic`)
      (set `self.Magnetic` false)
      (`PrimitiveComponent.SetMaterial` (`self.Magnet`) 0 "/Game/Materials/M_SouthPole.M_SouthPole")
      (else
        (set `self.Magnetic` true)
        (`PrimitiveComponent.SetMaterial` (`self.Magnet`) 0 "/Game/Materials/M_Blue_Emit.M_Blue_Emit")))))

(event `self.ReceiveTick`
  (params (DeltaSeconds :type "Float (single-precision)"))
  (bind _timeleft (`self.TimeLeft`))
  (`PhysicsConstraintComponent.SetLinearZLimit` (`self.PhysicsConstraint`) "LCM_Limited" (`self.CableLength`))
  ;[1 1 1] Magnetism
  (if (`self.Magnetic`)
    (`self.ApplyInfluence` (`self.Magnet`) (`self.ActionRange`) (`SphereComponent.GetScaledSphereRadius` (`self.ActionRange`))))
  ;[1 1 1] Count Down Seconds
  (`KismetSystemLibrary.Delay` 1.0)
  (set `self.TimeLeft` (- _timeleft 1))
  (if (== _timeleft 0)
    (`GameplayStatics.SetGamePaused` true)))

(fn `ApplyInfluence`
  (params (Magnet :type "PrimitiveComponent Object Reference") (ActionRange :type "PrimitiveComponent Object Reference") (MaxDistance :type "Float (double-precision)"))
  (locals (L_Pole :type "PrimitiveComponent Object Reference") (L_ForeignPole :type "PrimitiveComponent Object Reference") (L_ActionRange :type "PrimitiveComponent Object Reference") (L_MaxDistance :type "Float (double-precision)"))
  (bind _l_pole (`local.L_Pole`))
  (bind _l_maxdistance (`local.L_MaxDistance`))
  (bind _returnvalue (`PrimitiveComponent.GetCenterOfMass` (`local.L_ForeignPole`) "None"))
  (bind _returnvalue_2 (- (`PrimitiveComponent.GetCenterOfMass` _l_pole "None") _returnvalue))
  (set `local.L_Pole` Magnet)
  (set `local.L_ActionRange` ActionRange)
  (set `local.L_MaxDistance` MaxDistance)
  (for _array_element (`PrimitiveComponent.GetOverlappingComponents` (`local.L_ActionRange`))
    (bind _output_get (set `local.L_ForeignPole` _array_element))
    (if (!= _output_get _l_pole)
      (`PrimitiveComponent.AddForceAtLocation` (`local.L_ForeignPole`) (/ (* (* (`KismetMathLibrary.Normal` _returnvalue_2) (* (`self.MaxForce`) (`KismetMathLibrary.Square` (/ (- _l_maxdistance (`KismetMathLibrary.FClamp` (`KismetMathLibrary.VSize` _returnvalue_2) 0.0 _l_maxdistance)) _l_maxdistance)))) (select `bool` (!= (`PrimitiveComponent.GetMaterial` (`local.L_ForeignPole`) 0) (`PrimitiveComponent.GetMaterial` (`local.L_Pole`) 0)) :`false` -1.0 :`true` 1.0 :!type "Float (single-precision)")) 2.0) _returnvalue "None"))))

(fn `UserConstructionScript`)