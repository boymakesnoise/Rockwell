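; BP_PlayerControllerRW is a player controller that lets the player take control of a crane and return to the character.
; On BeginPlay it caches the BP_Player character reference.
; When that reference allows crane possession, the Use input alternates via a FlipFlop between possessing the first BP_Kran found, keeping the view target on the player, and re-possessing the first BP_Player found.
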(event `self.ReceiveBeginPlay`
  (bind _asbp_player (cast `/Game/Blueprints/BP_Player` (`GameplayStatics.GetPlayerCharacter` 0)))
  (set `self.PlayerReference` _asbp_player))

(event `InputAction|Use`
  (params (Key :type "Key Structure"))
  (:`Pressed`
    (if (`/Game/Blueprints/BP_Player.CanPossessCrane` (`self.PlayerReference`))
      (`/Engine/EditorBlueprintResources/StandardMacros.FlipFlop`
        (:`A`
          (bind _outactors (`GameplayStatics.GetAllActorsOfClass` "/Game/Blueprints/BP_Kran.BP_Kran_C"))
          (`self.Possess` (`|GetArrayItem` _outactors))
          (`self.SetViewTargetWithBlend` (`self.PlayerReference`)))
        (:`B`
          (bind _outactors_2 (`GameplayStatics.GetAllActorsOfClass` "/Game/Blueprints/BP_Player.BP_Player_C"))
          (`self.Possess` (`|GetArrayItem` _outactors_2)))))))

(fn `UserConstructionScript`)