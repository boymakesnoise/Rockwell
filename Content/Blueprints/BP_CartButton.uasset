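; BP_CartButton is an interactable button that changes the movement state of a referenced cart.
; Any actor overlap enables input from player 0, and ending the overlap disables it.
; Pressing Use adds the cart's SwitchDir, as a byte, to its MovementState, casts the sum back to E_CartDirection, and prints the new state.
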(event `self.ReceiveActorBeginOverlap`
  (params (OtherActor :type "Actor Object Reference"))
  ;[1 1 1] Take input from player?
  (`self.EnableInput` (`GameplayStatics.GetPlayerController` 0)))

(event `self.ReceiveActorEndOverlap`
  (params (OtherActor :type "Actor Object Reference"))
  ;[1 1 1] Take input from player?
  (`self.DisableInput` (`GameplayStatics.GetPlayerController` 0)))

(event `InputAction|Use`
  (params (Key :type "Key Structure"))
  (bind _cartreference (`self.CartReference`))
  (bind _movementstate (`/Game/Blueprints/BP_Cart.MovementState` _cartreference))
  (:`Pressed`
    (set `/Game/Blueprints/BP_Cart.MovementState` (cast `/Game/Blueprints/E_CartDirection` (+ _movementstate (`KismetMathLibrary.Conv_IntToByte` (`/Game/Blueprints/BP_Cart.SwitchDir` _cartreference)))) _cartreference)
    (`KismetSystemLibrary.PrintString` (`|GetEnumeratorNameAsString` _movementstate))))

(fn `UserConstructionScript`)